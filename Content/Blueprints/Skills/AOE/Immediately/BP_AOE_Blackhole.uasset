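; BP_AOE_Blackhole is an area-of-effect skill actor, a black hole that applies effects repeatedly over its lifetime.
; On BeginPlay it activates SkillVFX and starts two timers: a looping tick that calls CollectAndApplyEffects and a one-shot for Duration.
; At finish it spawns a dark impact effect at the collision sphere's relative location, applies effects once more and destroys itself.
; The finish-sound branch is unconnected and never runs.
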(event `self.ReceiveBeginPlay`
  (`ActorComponent.Activate` (`self.SkillVFX`) false)
  (`KismetSystemLibrary.K2_SetTimerDelegate` (delegate `IntervalEvent`) (`self.TickInterval`) true)
  (`KismetSystemLibrary.K2_SetTimerDelegate` (delegate `FinishEvent`) (`self.Duration`)))

(event `FinishEvent`
  (`NiagaraFunctionLibrary.SpawnSystemAtLocation` "/Game/_Externel_Asset/Mixed_Magic_VFX_Pack/VFX/NS_Dark_Solo_Impact.NS_Dark_Solo_Impact" (`SceneComponent.RelativeLocation` (`self.CollisionSphere`)))
  (`self.BP_CollectAndApplyEffects`)
  (`self.K2_DestroyActor`))

(event `IntervalEvent`
  (`self.BP_CollectAndApplyEffects`))

(fn `UserConstructionScript`)