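; Skill projectile actor that supplies visual and sound effects for the projectile and its hits, using soft asset references from its Config.
; On BeginPlay, after the parent logic, it async-loads and assigns the projectile VFX, then SFX, to their components, and starts preloading both hit assets.
; OnInstantHit spawns the pooled hit VFX at the target's location and plays the hit sound in 2D.
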(event `self.ReceiveBeginPlay`
  (bind (_actorclass _actortype _effects _spawnlocationpolicy _targetpolicy _speed _maxrange _lifespan _hitsperlifespan _radius _indicatordecalmaterial _montage _visualasset) (break `HeroSpawnableConfig` (`self.Config`)))
  (bind _projectilevfx (`DataAsset_SkillVisualData.ProjectileVFX` _visualasset))
  (bind _projectilesfx (`DataAsset_SkillVisualData.ProjectileSFX` _visualasset))
  (`parent.ReceiveBeginPlay`)
  (`|ExecutionSequence`
    (:`then_0`
      (bind _object (`|LoadAsset` _projectilevfx)
        (:`Completed`
          (`/Engine/EditorBlueprintResources/StandardMacros.IsValid` _object
            (:`Is Valid`
              (`NiagaraComponent.SetAsset` (`self.ActorVFXComponent`) (`|ConvertAsset` _projectilevfx) true)
              (bind _object_2 (`|LoadAsset` _projectilesfx)
                (:`Completed`
                  (`/Engine/EditorBlueprintResources/StandardMacros.IsValid` _object_2
                    (:`Is Valid`
                      (`AudioComponent.SetSound` (`self.ActorSFXComponent`) (`|ConvertAsset` _projectilesfx)))))))))))
    (:`then_1`
      (`|LoadAsset` (`DataAsset_SkillVisualData.HitVFX` _visualasset)
        (:`then`
          (`|LoadAsset` (`DataAsset_SkillVisualData.HitSFX` _visualasset)))))))

(event `self.OnInstantHit`
  (params (TargetActor :type "Actor Object Reference"))
  (bind (_actorclass _actortype _effects _spawnlocationpolicy _targetpolicy _speed _maxrange _lifespan _hitsperlifespan _radius _indicatordecalmaterial _montage _visualasset) (break `HeroSpawnableConfig` (`self.Config`)))
  (`NiagaraFunctionLibrary.SpawnSystemAtLocation` (`|ConvertAsset` (`DataAsset_SkillVisualData.HitVFX` _visualasset)) (`self.K2_GetActorLocation` TargetActor) (struct) (1.0 1.0 1.0) true true "AutoRelease")
  (`GameplayStatics.SpawnSound2D` (`|ConvertAsset` (`DataAsset_SkillVisualData.HitSFX` _visualasset)) 1.0 1.0 0.0 null))

(fn `UserConstructionScript`)