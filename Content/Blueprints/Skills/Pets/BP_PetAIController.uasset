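; AI controller for skill pets that runs the pet behavior tree on BeginPlay.
; On possess, it stores the pet and writes its Instigator to the ParentActor blackboard key.
; If the attribute set is valid, it copies AttackRange to the blackboard after a short delay.
; A one-shot attribute-change listener prints the new value but sets the AttackRange key to zero.
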(event `self.ReceiveBeginPlay`
  (`self.RunBehaviorTree` (`self.BTAsset`)))

(event `self.ReceivePossess`
  (params (PossessedPawn :type "Pawn Object Reference"))
  (bind (_attackrange_basevalue _attackrange_currentvalue) (break `GameplayAttributeData` (`PGCharacterAttributeSet.AttackRange` (`PGCharacterBase.CharacterAttributeSet` (`self.OwningPet`)))))
  (bind _aspet_character (cast `PetCharacter` PossessedPawn))
  (set `self.OwningPet` _aspet_character)
  (`BlackboardComponent.SetValueAsObject` (`AIBlueprintHelperLibrary.GetBlackboard` null) "ParentActor" (`self.GetInstigator` PossessedPawn))
  (`/Engine/EditorBlueprintResources/StandardMacros.IsValid` (`PGCharacterBase.CharacterAttributeSet` (`self.OwningPet`))
    (:`Is Valid`
      (`|ExecutionSequence`
        (:`then_0`
          (bind (_asynctaskproxy _attribute _newvalue) (`AbilityAsync_WaitAttributeChanged.WaitForAttributeChanged` null (struct :`AttributeName` "AttackRange" :`Attribute` "/Script/Unreal_ProjectG.PGCharacterAttributeSet:AttackRange" :`AttributeOwner` "/Script/CoreUObject.Class'/Script/Unreal_ProjectG.PGCharacterAttributeSet'") true)
            (:`Changed`
              (`KismetSystemLibrary.PrintString` (`KismetStringLibrary.BuildString_Double` "" "" _newvalue))
              (`BlackboardComponent.SetValueAsFloat` (`AIBlueprintHelperLibrary.GetBlackboard` null) "AttackRange" 0.0))))
        (:`then_1`
          (`KismetSystemLibrary.Delay` 0.1)
          (`BlackboardComponent.SetValueAsFloat` (`AIBlueprintHelperLibrary.GetBlackboard` null) "AttackRange" _attackrange_currentvalue))))))

(fn `UserConstructionScript`)