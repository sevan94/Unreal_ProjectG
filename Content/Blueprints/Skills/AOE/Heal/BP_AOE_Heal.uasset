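; BP_AOE_Heal is a one-shot area-of-effect heal skill actor that does all its work on BeginPlay.
; It spawns an auto-released pooled heal VFX at its collision sphere and calls CollectAndApplyEffects with the skill multiplier.
; It then executes the shared HealCast gameplay cue on each overlapped target, crediting the instigator, and destroys itself.
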(event `self.ReceiveBeginPlay`
  (bind _instigatoractor (`self.InstigatorActor`))
  (`NiagaraFunctionLibrary.SpawnSystemAtLocation` (`self.HealVFX`) (`SceneComponent.K2_GetComponentLocation` (`self.CollisionSphere`)) (struct) (1.0 1.0 1.0) true true "AutoRelease")
  (`self.BP_CollectAndApplyEffects` (`self.SkillMultiplier`))
  (for _array_element (`self.GetOverlappedTargets`)
    (`GameplayCueFunctionLibrary.ExecuteGameplayCueOnActor` _array_element (struct :`TagName` "GameplayCue.SVFX.Shared.HealCast") (`AbilitySystemBlueprintLibrary.MakeGameplayCueParameters` 0.0 0.0 (struct) (struct) (struct) (struct) (struct) (0.0 0.0 0.0) (0.0 0.0 0.0) _instigatoractor _instigatoractor)))
  (`self.K2_DestroyActor`))

(fn `UserConstructionScript`)