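; Upgraded black hole area-of-effect skill actor that pulls targets inward, deals repeated hits, then finishes with a final burst.
; Tick lerps every overlapped target toward the collision sphere's center, scaled by delta time.
; A looping timer, spaced by level-scaled duration divided by hit count, applies tick-multiplier effects.
; Once the count exceeds the hit count, it spawns finish VFX, applies the final skill multiplier and destroys itself.
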(event `self.ReceiveBeginPlay`
  (`KismetSystemLibrary.K2_SetTimerDelegate` (delegate `OnTick`) (`self.GetTickInterval`) true))

(event `OnTick`
  (if (<= (`self.CurrentHitCount`) (`self.GetScalableValueAtLevel` (`self.HitCount`)))
    (`self.BP_CollectAndApplyEffects` (`self.GetScalableValueAtLevel` (`self.BlackholeTickSkillMultiplier`)))
    (`/Engine/EditorBlueprintResources/StandardMacros.IncrementFloat` (`self.CurrentHitCount`))
    (else
      (`NiagaraFunctionLibrary.SpawnSystemAtLocation` (`self.BlackholeFinishVFX`) (`SceneComponent.K2_GetComponentLocation` (`self.CollisionSphere`)) (struct) (3.0 3.0 3.0) true true "AutoRelease")
      (`self.BP_CollectAndApplyEffects` (`self.GetScalableValueAtLevel` (`self.BlakcholeSkillMultiplier`)))
      (`self.K2_DestroyActor`))))

(event `self.ReceiveTick`
  (params (DeltaSeconds :type "Float (single-precision)"))
  (bind _returnvalue (`self.GetOverlappedTargets`))
  (if (`KismetArrayLibrary.Array_IsNotEmpty` _returnvalue)
    (for _array_element _returnvalue
      (`self.K2_SetActorLocation` _array_element (`KismetMathLibrary.VLerp` (`self.K2_GetActorLocation` _array_element) (`SceneComponent.K2_GetComponentLocation` (`self.CollisionSphere`)) (* DeltaSeconds 1.0)) false false))))

(fn `GetTickInterval`
  (returns (OutTickInterval :type "Float (double-precision)"))
  (return (/ (`self.GetScalableValueAtLevel` (`self.BlackholeDuration`)) (`self.GetScalableValueAtLevel` (`self.HitCount`)))))

(fn `UserConstructionScript`)