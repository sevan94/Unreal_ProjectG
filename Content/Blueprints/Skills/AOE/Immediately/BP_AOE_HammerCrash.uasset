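; BP_AOE_HammerCrash is an immediate area-of-effect skill actor for Hammer Crash that resolves entirely on BeginPlay and then destroys itself.
; It collects and applies effects using the level-scaled finish skill multiplier, then spawns the pooled finish VFX at the collision sphere.
; A long-lived debug sphere with a hardcoded radius is still drawn there.
; The finish-sound logic is disconnected and never runs.
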(event `self.ReceiveBeginPlay`
  (bind _returnvalue (`SceneComponent.K2_GetComponentLocation` (`self.CollisionSphere`)))
  (`self.BP_CollectAndApplyEffects` (`self.GetScalableValueAtLevel` (`self.FinishSkillMultiplier`)))
  (`NiagaraFunctionLibrary.SpawnSystemAtLocation` (`self.FinishVFX`) _returnvalue (struct) (1.0 1.0 1.0) true true "AutoRelease")
  (`KismetSystemLibrary.DrawDebugSphere` _returnvalue 200.0 12 (struct :`R` 1.0 :`G` 1.0 :`B` 1.0 :`A` 1.0) 100.0 1.0)
  (`self.K2_DestroyActor`))

(fn `UserConstructionScript`)