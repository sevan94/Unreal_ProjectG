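; Persistent ground fire AOE skill actor that supplies the looping presentation on top of its parent skill actor class.
; On BeginPlay it snaps onto its owner, keeping world scale, then async-loads the persistent VFX and SFX from Config into its components.
; Each OnTickforOwner event activates the VFX with a reset and prints a leftover "Hello" debug string.
; Overlap, damage and timing logic are absent from this graph.
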(event `self.ReceiveBeginPlay`
  (bind (_actorclass _actortype _effects _spawnlocationpolicy _targetpolicy _speed _maxrange _lifespan _hitsperlifespan _radius _indicatordecalmaterial _montage _visualasset) (break `HeroSpawnableConfig` (`self.Config`)))
  (bind _persistentvfx (`DataAsset_SkillVisualData.PersistentVFX` _visualasset))
  (bind _persistentsfx (`DataAsset_SkillVisualData.PersistentSFX` _visualasset))
  (`parent.ReceiveBeginPlay`)
  (`self.K2_AttachToActor` (`self.GetOwner`) "None" "SnapToTarget" "SnapToTarget" "KeepWorld")
  (`|ExecutionSequence`
    (:`then_0`
      (bind _object (`|LoadAsset` _persistentvfx)
        (:`Completed`
          (`/Engine/EditorBlueprintResources/StandardMacros.IsValid` _object
            (:`Is Valid`
              (`NiagaraComponent.SetAsset` (`self.ActorVFXComponent`) (`|ConvertAsset` _persistentvfx) true))))))
    (:`then_1`
      (`|LoadAsset` _persistentsfx
        (:`Completed`
          (`AudioComponent.SetSound` (`self.ActorSFXComponent`) (`|ConvertAsset` _persistentsfx)))))))

(event `self.OnTickForOwner`
  (params (TargetActor :type "Actor Object Reference"))
  (`ActorComponent.Activate` (`self.ActorVFXComponent`) true)
  (`KismetSystemLibrary.PrintString` "Hello"))

(fn `UserConstructionScript`
  (`parent.UserConstructionScript`))