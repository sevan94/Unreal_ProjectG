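; Thunder area-of-effect skill actor that strikes immediately when spawned and then removes itself.
; On BeginPlay it spawns an auto-release pooled thunder VFX at its location, applies effects through CollectAndApplyEffects using the level-scaled thunder multiplier, and destroys itself.
; An alternative path that waits for SkillVFX to finish before applying effects is left unconnected, as is the finish sound.
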(event `self.ReceiveBeginPlay`
  (`NiagaraFunctionLibrary.SpawnSystemAtLocation` (`self.ThunderVFX`) (`self.K2_GetActorLocation`) (struct) (1.0 1.0 1.0) true true "AutoRelease")
  (`self.BP_CollectAndApplyEffects` (`self.GetScalableValueAtLevel` (`self.ThunderSkillMultiplier`)))
  (`self.K2_DestroyActor`))

(event `OnSystemFinished_이벤트`
  (params (PSystem :type "NiagaraComponent Object Reference"))
  (`self.BP_CollectAndApplyEffects` (`self.GetScalableValueAtLevel` (`self.ThunderSkillMultiplier`)))
  (`self.K2_DestroyActor`))

(fn `UserConstructionScript`)