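; Blackhole area-of-effect skill actor that acts as a one-shot burst when spawned.
; On BeginPlay it spawns the blackhole finish VFX at its collision sphere, calls CollectAndApplyEffects with a level-scaled skill multiplier, then destroys itself immediately.
; A finish-sound branch exists but is not wired to any event, so it never plays.
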(event `self.ReceiveBeginPlay`
  (`NiagaraFunctionLibrary.SpawnSystemAtLocation` (`self.BlackholeFinishVFX`) (`SceneComponent.K2_GetComponentLocation` (`self.CollisionSphere`)) (struct) (2.0 2.0 2.0) true true "AutoRelease")
  (`self.BP_CollectAndApplyEffects` (`self.GetScalableValueAtLevel` (`self.BlakcholeSkillMultiplier`)))
  (`self.K2_DestroyActor`))

(fn `UserConstructionScript`)